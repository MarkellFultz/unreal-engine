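; BP_Food_Apple is an apple food actor that builds a procedural version of its mesh at runtime.
; On BeginPlay it copies the Applesouce static mesh component into a ProceduralMesh component with collision enabled, then assigns a material to the second element slot.
; The file contains no other active gameplay logic, and its construction script only calls the parent.
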(event EventBeginPlay
  (Class|KismetProceduralMeshLibrary|CopyProceduralMeshfromStaticMeshComponent (Variables|Default|Getapplesouce) 0 (Variables|Default|GetProceduralMesh) true)
  (Rendering|Material|SetMaterial (Variables|Default|GetProceduralMesh) 1 "/Game/Fab/Megascans/3D/Red_Apple_tgzoahbpa/Medium/tgzoahbpa_tier_2/Materials/MI_tgzoahbpa.MI_tgzoahbpa"))

(event Collision|EventActorBeginOverlap
  (params (OtherActor :type Actor%20Object%20Reference))
  (|CallParentFunction OtherActor) ; This node is disabled and will not be called.\nDrag off pins to build functionality.
)

(event EventTick
  (params (DeltaSeconds :type Float%20%28single-precision%29))
  (|CallParentFunction DeltaSeconds) ; This node is disabled and will not be called.\nDrag off pins to build functionality.
)

(fn ConstructionScript
  (|CallParentFunction))