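; Airfryer actor that serves as a cooking station with a sliding drawer and ingredient selection.
; Drawer interaction alternates a timeline that slides the tray out or back and activates smoke.
; Opening the cooking UI spawns WBP_Inventory targeting this fryer and blocks player movement.
; A chosen ingredient is looked up in DT_Ingredients, spawned as a mesh on the tray, passed to AcceptIngredients, and move/look input is restored.
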(event Custom|InteractDrawer
  (bind _initialtraylocation (Variables|Default|GetInitialTrayLocation))
  (Utilities|FlowControl|FlipFlop
    (:A
      (bind _newtrack_0 (Timeline|DrawerTimeline PlayFromStart)
        (:Update
          (Components|Activation|Activate (Variables|Default|GetSmokeEffect) false)
          (Transformation|SetRelativeLocation (Variables|Default|GetSM_AirfryerTray) (Math|Vector|Lerp(Vector) _initialtraylocation (+ _initialtraylocation "0.000000,20.000000,0.000000") _newtrack_0) false false))))
    (:B
      (Timeline|DrawerTimeline Reverse))))

(event EventBeginPlay
  (Variables|Default|SetInitialTrayLocation (Variables|/Script/Engine.SceneComponent|GetRelativeLocation (Variables|Default|GetSM_AirfryerTray))))

(event Collision|EventActorBeginOverlap
  (params (OtherActor :type Actor%20Object%20Reference)))

(event EventIngredient
  (params (IngredientID :type Name :default "None") (Interactor :type Actor%20Object%20Reference))
  (bind _returnvalue (Utilities|GetDataTableRow "/Game/DataTable/DT_Ingredients.DT_Ingredients" IngredientID)
    (:then
      (bind _output_get (Variables|Default|SetCurrentIngredientData _returnvalue))
      (bind _returnvalue_2 (AddComponent|AddStaticMeshComponent true (Math|Transform|MakeTransform "0.000000,-15.000000,-3.000000" "0, 0, 0" "1.000000,1.000000,1.000000")))
      (Transformation|AttachComponentToComponent _returnvalue_2 (Variables|Default|GetSM_AirfryerTray) "None" "KeepRelative" "KeepRelative" "KeepRelative" true)
      (Variables|Default|SetCurrentFoodMesh _returnvalue_2)
      (Components|StaticMesh|SetStaticMesh _returnvalue_2 (Utilities|ResolveSoftReference (.IngredientMesh (Utilities|Struct|BreakIngredientData _output_get))))
      (Class|CookingToolActor|AcceptIngredients Interactor (Utilities|Array|MakeArray IngredientID))
      (bind _returnvalue_3 (Class|InputDeviceLibrary|GetPlayerControllerfromInputDevice))
      (Input|SetIgnoreMoveInput _returnvalue_3 false)
      (Input|SetIgnoreLookInput _returnvalue_3 false))))

(event EventTick
  (params (DeltaSeconds :type Float%20%28single-precision%29)))

(event EventOnOpenCookingUI
  (params (Interactor :type Actor%20Object%20Reference))
  (bind _asmy_character (Utilities|Casting|CastToMyCharacter Interactor))
  (Class|MyCharacter|SetUIInputMode _asmy_character true)
  (bind _returnvalue (UserInterface|CreateWidget "/Game/Blueprints/WBP_Inventory.WBP_Inventory_C" 0 self))
  (UserInterface|Viewport|AddtoViewport _returnvalue 0)
  (bind _returnvalue_2 (Class|InputDeviceLibrary|GetPlayerControllerfromInputDevice))
  (Input|SetIgnoreMoveInput _returnvalue_2 true))

(fn ConstructionScript)