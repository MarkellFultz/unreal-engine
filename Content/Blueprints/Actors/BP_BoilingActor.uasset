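; BP_BoilingActor is a boiling cooking station that runs ingredient selection, a QTE and a result screen.
; Opening it switches the interacting character to UI input, locks movement and shows the inventory widget targeting the station.
; QTE start and finish toggle fire particles and spawn the QTE and result widgets, while ingredient events forward to AcceptIngredients.
; A stir timeline rotates the ladle and drives the water material's panner speed.
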(event Custom|stir
  (bind (_direction _spoonrotationtrack _waterspeedtrack) (Timeline|StirVisualTimeline PlayFromStart)
    (:Update
      (Transformation|SetRelativeRotation (Variables|Default|GetLadleMesh) (Math|Rotator|MakeRotator 0.0 0.0 _spoonrotationtrack) false false)
      (Rendering|Material|SetScalarParameterValueonMaterials (Variables|Default|GetWaterMesh) "PannerSpeed" _waterspeedtrack))))

(event EventBeginPlay)

(event Collision|EventActorBeginOverlap
  (params (OtherActor :type Actor%20Object%20Reference)))

(event EventTick
  (params (DeltaSeconds :type Float%20%28single-precision%29)))

(event EventOnQTEStarted
  (Components|Activation|Activate (Variables|Default|GetFireParticles) true)
  (bind _returnvalue (UserInterface|CreateWidget "/Game/Blueprints/WBP_QTE.WBP_QTE_C" 0 (Variables|Default|GetQTEComp) self))
  (UserInterface|Viewport|AddtoViewport _returnvalue 0))

(event EventOnOpenCookingUI
  (params (Interactor :type Actor%20Object%20Reference))
  (bind _asmy_character (Utilities|Casting|CastToMyCharacter Interactor))
  (Class|MyCharacter|SetUIInputMode _asmy_character true)
  (bind _returnvalue (UserInterface|CreateWidget "/Game/Blueprints/WBP_Inventory.WBP_Inventory_C" 0 self))
  (UserInterface|Viewport|AddtoViewport _returnvalue 0)
  (bind _returnvalue_2 (Class|InputDeviceLibrary|GetPlayerControllerfromInputDevice))
  (Input|SetIgnoreMoveInput _returnvalue_2 true))

(event EventOnCookingFinished
  (params (FinalSuccessCount :type Integer))
  (Components|Activation|Deactivate (Variables|Default|GetFireParticles))
  (bind _returnvalue (UserInterface|CreateWidget "/Game/Blueprints/WBP_CookingResult.WBP_CookingResult_C" 0 FinalSuccessCount))
  (UserInterface|Viewport|AddtoViewport _returnvalue 0)
  (bind _asmy_character (Utilities|Casting|CastToMyCharacter (Game|GetPlayerCharacter 0)))
  (Class|MyCharacter|SetUIInputMode _asmy_character true))

(event EventIngredient
  (params (IngredientID :type Name :default "None") (Interactor :type Actor%20Object%20Reference))
  (Class|CookingToolActor|AcceptIngredients Interactor (Utilities|Array|MakeArray IngredientID)))

(fn ConstructionScript)