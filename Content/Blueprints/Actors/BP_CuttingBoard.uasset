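; Cutting board actor that lets a character pick an ingredient from an inventory UI to place on it.
; On the open-inventory event it creates WBP_Inventory, registers itself as both cooking and cutting target, and switches the interacting MyCharacter to UI input mode.
; The Ingredient event forwards the ingredient ID and interactor to PlaceIngredient, whose logic lives outside this graph.
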(event EventBeginPlay)

(event Collision|EventActorBeginOverlap
  (params (OtherActor :type Actor%20Object%20Reference)))

(event EventTick
  (params (DeltaSeconds :type Float%20%28single-precision%29)))

(event EventOnOpenInventoryUI
  (params (Interactor :type Actor%20Object%20Reference))
  (bind _self self)
  (bind _returnvalue (UserInterface|CreateWidget "/Game/Blueprints/WBP_Inventory.WBP_Inventory_C" 0 0 "None" 0))
  (Variables|/Game/Blueprints/WBP_Inventory.WBP_Inventory_C|SetCookingTarget _returnvalue _self)
  (Variables|/Game/Blueprints/WBP_Inventory.WBP_Inventory_C|SetCuttingtarget _returnvalue _self)
  (UserInterface|Viewport|AddtoViewport _returnvalue 0)
  (bind _asmy_character (Utilities|Casting|CastToMyCharacter Interactor))
  (Class|MyCharacter|SetUIInputMode _asmy_character true))

(event EventIngredient
  (params (IngredientID :type Name :default "None") (Interactor :type Actor%20Object%20Reference))
  (Class|CuttingBoardActor|PlaceIngredient IngredientID Interactor))

(fn ConstructionScript)