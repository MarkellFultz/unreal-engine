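; Frying pan cooking station that runs a quick-time-event cooking minigame for a player holding a spatula.
; Opening it shows an inventory widget; the chosen ingredient's DT_Ingredients mesh spawns in the pan as the camera blends over and the spatula visual swaps.
; QTE successes toss and rotate the food through a Timeline.
; Finishing shows a result widget, returns the camera, re-enables movement input and reattaches the held actor to the player's SpatulaHolder.
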(event OnQTECompleted(QTEComp)
  (params (bWasSuccessful :type Boolean))
  (bind _currentfoodmesh (Variables|Default|GetCurrentFoodMesh))
  (bind _currentfoodmesh_2 (Variables|Default|GetCurrentFoodMesh))
  (if bWasSuccessful
    (Physics|SetSimulatePhysics _currentfoodmesh false)
    (bind _output_get (Variables|Default|SetStartLoc (Variables|/Script/Engine.SceneComponent|GetRelativeLocation _currentfoodmesh)))
    (bind _output_get_2 (Variables|Default|SetStartRot (Variables|/Script/Engine.SceneComponent|GetRelativeRotation _currentfoodmesh)))
    (bind _output_get_3 (Variables|Default|SetEndRot (Math|Rotator|CombineRotators _output_get_2 (Math|Conversions|RotationFromXVector _output_get))))
    (bind (_direction _z_height _alpha) (Timeline|Timeline PlayFromStart)
      (:Update
        (Transformation|SetRelativeLocationAndRotation _currentfoodmesh_2 (Math|Vector|MakeVector (.x (Variables|Default|GetStartLoc)) (.y (Variables|Default|GetStartLoc)) (+ (.z (Variables|Default|GetStartLoc)) _z_height)) (Math|Rotator|Lerp(Rotator) _output_get_2 _output_get_3 _alpha true) false false))
      (:Finished
        (Physics|SetSimulatePhysics _currentfoodmesh_2 false)))))

(event EventBeginPlay)

(event Collision|EventActorBeginOverlap
  (params (OtherActor :type Actor%20Object%20Reference)))

(event EventTick
  (params (DeltaSeconds :type Float%20%28single-precision%29)))

(event EventOnCookingFinished
  (params (FinalSuccessCount :type Integer))
  (bind _returnvalue (Game|GetPlayerController 0))
  (bind _returnvalue_2 (UserInterface|CreateWidget "/Game/Blueprints/WBP_CookingResult.WBP_CookingResult_C" 0 FinalSuccessCount))
  (UserInterface|Viewport|AddtoViewport _returnvalue_2 0)
  (bind _asmy_character (Utilities|Casting|CastToMyCharacter (Game|GetPlayerCharacter 0)))
  (Class|MyCharacter|SetUIInputMode _asmy_character true)
  (Game|Player|SetViewTargetwithBlend _returnvalue (Game|GetPlayerCharacter 0) 0.5 "VTBlend_Linear" 0.0 false)
  (Input|SetIgnoreMoveInput _returnvalue false)
  (bind _asbp_first_person_character (Utilities|Casting|CastToBP_FirstPersonCharacter (Game|GetPlayerCharacter 0)))
  (Transformation|AttachComponentToComponent (Variables|/Game/FirstPerson/Blueprints/BP_FirstPersonCharacter.BP_FirstPersonCharacter_C|GetHeldActor _asbp_first_person_character) (Variables|/Game/FirstPerson/Blueprints/BP_FirstPersonCharacter.BP_FirstPersonCharacter_C|GetSpatula_Holder _asbp_first_person_character) "None" "SnapToTarget" "SnapToTarget" "SnapToTarget" true)
  (Rendering|SetVisibility (Variables|Default|GetCookingSpatula) false false))

(event EventIngredient
  (params (IngredientID :type Name :default "None") (Interactor :type Actor%20Object%20Reference))
  (bind _returnvalue (Utilities|GetDataTableRow "/Game/DataTable/DT_Ingredients.DT_Ingredients" IngredientID)
    (:then
      (bind _output_get (Variables|Default|SetCurrentIngredientData _returnvalue))
      (bind _returnvalue_2 (AddComponent|AddStaticMeshComponent false (Math|Transform|MakeTransform "0.000000,0.000000,10.000000" "0, 0, 0" "5.000000,5.000000,5.000000")))
      (Variables|Default|SetCurrentFoodMesh _returnvalue_2)
      (Components|StaticMesh|SetStaticMesh _returnvalue_2 (Utilities|ResolveSoftReference (.IngredientMesh (Utilities|Struct|BreakIngredientData _output_get))))
      (Class|CookingToolActor|AcceptIngredients Interactor (Utilities|Array|MakeArray IngredientID))
      (Game|Player|SetViewTargetwithBlend (Game|GetPlayerController 0) self 0.5 "VTBlend_Linear" 0.0 false)
      (bind _asbp_first_person_character (Utilities|Casting|CastToBP_FirstPersonCharacter Interactor))
      (Rendering|SetVisibility (Variables|/Game/FirstPerson/Blueprints/BP_FirstPersonCharacter.BP_FirstPersonCharacter_C|GetSpatula_Holder _asbp_first_person_character) false false)
      (Rendering|SetVisibility (Variables|Default|GetCookingSpatula) true false))))

(event EventOnQTEStarted
  (bind _returnvalue (UserInterface|CreateWidget "/Game/Blueprints/WBP_QTE.WBP_QTE_C" 0 (Variables|Default|GetQTEComp) self))
  (UserInterface|Viewport|AddtoViewport _returnvalue 0))

(event EventOnOpenCookingUI
  (params (Interactor :type Actor%20Object%20Reference))
  (bind _asbp_first_person_character (Utilities|Casting|CastToBP_FirstPersonCharacter Interactor))
  (Utilities|Casting|CastTospatula (Variables|/Game/FirstPerson/Blueprints/BP_FirstPersonCharacter.BP_FirstPersonCharacter_C|GetHeldActor _asbp_first_person_character))
  (if true
    (bind _asmy_character (Utilities|Casting|CastToMyCharacter Interactor))
    (Class|MyCharacter|SetUIInputMode _asmy_character true)
    (bind _returnvalue (UserInterface|CreateWidget "/Game/Blueprints/WBP_Inventory.WBP_Inventory_C" 0 self))
    (UserInterface|Viewport|AddtoViewport _returnvalue 0)
    (bind _returnvalue_2 (Class|InputDeviceLibrary|GetPlayerControllerfromInputDevice))
    (Input|SetIgnoreMoveInput _returnvalue_2 true)))

(fn ConstructionScript)