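; Chicken breast food actor that can flip itself over, likely for a cooking interaction.
; FlipFood switches off physics on the mesh and stores its relative location and rotation as the starting pose.
; The FlipAnim timeline then lifts it along a height curve while lerping through a half-turn.
; Physics simulation switches back on when the timeline finishes.
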(event EventBeginPlay)

(event Collision|EventActorBeginOverlap
  (params (OtherActor :type Actor%20Object%20Reference)))

(event EventTick
  (params (DeltaSeconds :type Float%20%28single-precision%29)))

(event EventFlipFood
  (bind _chickenbreast (Variables|Default|GetChickenBreast))
  (bind _chickenbreast_2 (Variables|Default|GetChickenBreast))
  (Physics|SetSimulatePhysics _chickenbreast false)
  (bind _output_get (Variables|Default|SetStartLoc (Variables|/Script/Engine.SceneComponent|GetRelativeLocation _chickenbreast)))
  (bind _output_get_2 (Variables|Default|SetStartRot (Variables|/Script/Engine.SceneComponent|GetRelativeRotation _chickenbreast)))
  (bind _output_get_3 (Variables|Default|SetEndRot (Math|Rotator|CombineRotators _output_get_2 "180.000000,0.000000,0.000000")))
  (bind (_direction _z_height _alpha) (Timeline|FlipAnim PlayFromStart)
    (:Update
      (Transformation|SetRelativeLocationAndRotation _chickenbreast_2 (Math|Vector|MakeVector (.x (Variables|Default|GetStartLoc)) (.y (Variables|Default|GetStartLoc)) (+ (.z (Variables|Default|GetStartLoc)) _z_height)) (Math|Rotator|Lerp(Rotator) _output_get_2 _output_get_3 _alpha true) false false))
    (:Finished
      (Physics|SetSimulatePhysics _chickenbreast_2 true))))

(fn ConstructionScript)