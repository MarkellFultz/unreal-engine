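; Air fryer appliance Blueprint with a tray drawer that slides open and closed on interaction.
; BeginPlay activates the smoke effect and caches the tray mesh's starting relative location.
; InteractDrawer uses a FlipFlop to play or reverse a timeline, which lerps the tray between that location and a fixed offset along local Y.
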(event Custom|InteractDrawer
  (bind _initialtraylocation (Variables|Default|GetInitialTrayLocation))
  (Utilities|FlowControl|FlipFlop
    (:A
      (bind _newtrack_0 (Timeline|DrawerTimeline Play)
        (:Update
          (Transformation|SetRelativeLocation (Variables|Default|GetSM_KA_Airfryer_V1_Tray) (Math|Vector|Lerp(Vector) _initialtraylocation (+ _initialtraylocation "0.000000,20.000000,0.000000") _newtrack_0) false false))))
    (:B
      (Timeline|DrawerTimeline Reverse))))

(event EventBeginPlay
  (Components|Activation|Activate (Variables|Default|GetSmokeEffect) false)
  (Variables|Default|SetInitialTrayLocation (Variables|/Script/Engine.SceneComponent|GetRelativeLocation (Variables|Default|GetSM_KA_Airfryer_V1_Tray))))

(event Collision|EventActorBeginOverlap
  (params (OtherActor :type Actor%20Object%20Reference)))

(event EventTick
  (params (DeltaSeconds :type Float%20%28single-precision%29)))

(fn ConstructionScript)