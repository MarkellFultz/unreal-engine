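; BP_CustomerNPC is an interactable customer in a cooking game that triggers an order when the player interacts with it.
; Interact reads the selected customer row name from GI_CookingGame and passes it to ReceiveOrder on the OrderManagerComponent of BP_GameMode.
; The event graph holds only disabled events and unconnected logic for showing a WBP_OrderCard with UI-only input, which never runs.
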(event EventBeginPlay)

(event Collision|EventActorBeginOverlap
  (params (OtherActor :type Actor%20Object%20Reference)))

(event EventTick
  (params (DeltaSeconds :type Float%20%28single-precision%29)))

(fn ConstructionScript)

(fn Interact
  (Development|PrintString "\"Interact triggered\"")
  (bind _asgi_cooking_game (Utilities|Casting|CastToGI_CookingGame (Game|GetGameInstance)))
  (bind _asbp_game_mode (Utilities|Casting|CastToBP_GameMode (Game|GetGameMode))
    (:then
      (Class|OrderManagerComponent|ReceiveOrder (Actor|GetComponentbyClass _asbp_game_mode "/Script/MyProject.OrderManagerComponent") (Variables|/Game/Blueprints/GI_CookingGame.GI_CookingGame_C|GetSelectedCustomerRowName _asgi_cooking_game))
      (return 0))
    (:CastFailed
      (Development|PrintString "cast faield"))))