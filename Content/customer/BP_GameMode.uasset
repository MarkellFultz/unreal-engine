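; Game mode for the cooking game that records how long the selected customer's level takes to complete.
; BeginPlay casts to GI_CookingGame and looks up the selected customer in DT_Customerpr, though the fetched row is not used.
; OnLevelComplete loads PlayerSaveSlot, stores game time minus Startime in the LevelTimes map under that customer's row name, and saves.
; Startime is never set in this graph.
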(event Custom|OnLevelComplete
  (bind _returnvalue (SaveGame|LoadGamefromSlot "PlayerSaveSlot"))
  (bind _asmy_save_game (Utilities|Casting|CastToMySaveGame _returnvalue))
  (Utilities|Map|Add (Variables|/Script/MyProject.MySaveGame|GetLevelTimes _asmy_save_game) (Variables|/Game/Blueprints/GI_CookingGame.GI_CookingGame_C|GetSelectedCustomerRowName (stale EventBeginPlay _asgi_cooking_game)) (- (Utilities|Time|GetGameTimeinSeconds) (Variables|Default|GetStartime)))
  (SaveGame|SaveGametoSlot _asmy_save_game "PlayerSaveSlot"))

(event EventTick
  (params (DeltaSeconds :type Float%20%28single-precision%29)))

(event EventBeginPlay
  (bind _asgi_cooking_game (Utilities|Casting|CastToGI_CookingGame (Game|GetGameInstance)))
  (if (not (== (Variables|/Game/Blueprints/GI_CookingGame.GI_CookingGame_C|GetSelectedCustomerRowName _asgi_cooking_game) ""))
    (bind _returnvalue (Utilities|GetDataTableRow "/Game/DataTable/DT_Customerpr.DT_Customerpr" (Variables|/Game/Blueprints/GI_CookingGame.GI_CookingGame_C|GetSelectedCustomerRowName _asgi_cooking_game)))))

(fn ConstructionScript)